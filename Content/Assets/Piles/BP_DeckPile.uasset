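; BP_DeckPile is the deck pile actor in a card game, which supplies the commands available on it to the game board.
; GetCommands returns a reshuffle-deck command when its card pile component is empty and a draw-card command otherwise, whichever actor requests it.
; The pile opts out of drag and drop, offering no payload or drop command and refusing all incoming payloads.
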(event EventBeginPlay)

(event Collision|EventActorBeginOverlap
  (params (OtherActor :type Actor%20Object%20Reference)))

(event EventTick
  (params (DeltaSeconds :type Float%20%28single-precision%29)))

(fn ConstructionScript)

(fn GetCommands
  (params (GameBoard :type Solitaire%20Board%20Object%20Reference) (RequestingActor :type Actor%20Object%20Reference))
  ;[0 0 0] Same behaviour regardless of whether there is a requesting actor or none
  (if (Class|CardPileComponent|IsEmpty (Variables|Default|GetCardPileComponent))
    ;;[0 0 0] Reshuffle the deck if it is empty
    (bind _returnvalue (Game|ConstructObjectfromClass "/Game/Assets/Commands/BP_Command_ReshuffleDeck.BP_Command_ReshuffleDeck_C" GameBoard))
    (return (Utilities|Array|MakeArray _returnvalue))
    (else
      ;;[0 0 0] Draw a card otherwise
      (bind _returnvalue_2 (Game|ConstructObjectfromClass "/Game/Assets/Commands/BP_Command_DrawCard.BP_Command_DrawCard_C" GameBoard))
      (return (Utilities|Array|MakeArray _returnvalue_2)))))

(fn GetCommandDragDrop
  (params (GameBoard :type Solitaire%20Board%20Object%20Reference) (Payload_NEW :type Drag%20Drop%20Payload%20Object%20Reference) (RequestingActor :type Actor%20Object%20Reference))
  ;[0 0 0] No drag-and-drop commands for the deck pile
  (return 0))

(fn GetDragDropPayload
  (params (GameBoard :type Solitaire%20Board%20Object%20Reference) (RequestingActor :type Actor%20Object%20Reference))
  ;[0 0 0] Discard pile cards cannot be dragged
  (return 0))

(fn CanAcceptPayload
  (params (GameBoard :type Solitaire%20Board%20Object%20Reference) (Payload :type Drag%20Drop%20Payload%20Object%20Reference) (RequestingActor :type Actor%20Object%20Reference))
  ;[0 0 0] Deck pile cannot accept payloads
  (return false))