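; Tableau pile for a solitaire card game that turns card interactions and drag-and-drop into command objects.
; A face-down top card yields a flip command, while a face-up card yields transfer commands to every tableau and foundation pile that accepts it.
; Drag payloads carry the face-up card plus the cards on top of it.
; Drop validation defers to the card pile component's ruleset.
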(event EventBeginPlay)

(event Collision|EventActorBeginOverlap
  (params (OtherActor :type Actor%20Object%20Reference)))

(event EventTick
  (params (DeltaSeconds :type Float%20%28single-precision%29)))

(fn ConstructionScript)

(fn GetCommands
  (params (GameBoard :type Solitaire%20Board%20Object%20Reference) (RequestingActor :type Actor%20Object%20Reference))
  (bind _ascard (Utilities|Casting|CastToCard RequestingActor))
  (bind _output_get (LocalVariables|SetRequestingCard _ascard))
  (if (Variables|/Script/Cards.Card|GetbIsFaceDown _output_get)
    ;[0 0 0] If the card is face down...
    (if (== (Class|CardPileComponent|TopCard (Variables|Default|GetCardPileComponent)) (LocalVariables|GetRequestingCard))
      ;;[0 0 0] ... flip it over if it's the top card of the pile
      (bind _returnvalue (Game|ConstructObjectfromClass "/Script/Cards.CommandFlipCard" (LocalVariables|GetRequestingCard)))
      (return (Utilities|Array|MakeArray _returnvalue))
      (else
        ;;[0 0 0] ... do nothing otherwise
        (return 0)))
    (else
      ;[0 0 0] If the card is face up, make the card payload...
      (bind _ascard_payload (Utilities|Casting|CastToCardPayload (Class|InteractionInterface|GetDragDropPayload GameBoard RequestingActor)))
      (LocalVariables|SetCard%20Payload _ascard_payload)
      ;[0 0 0] ...and find all possible transfers for the payload
      (Utilities|FlowControl|Sequence
        (:then_0
          ;;[0 0 0] Create card transfer commands to the tableau piles
          (for _array_element (Class|SolitaireBoard|GetTableau GameBoard)
            (bind _output_get_2 (LocalVariables|SetDestination (Variables|/Script/Cards.CardPile|GetCardPileComponent _array_element)))
            (if (Class|CardPileComponent|CanAccept _output_get_2 (LocalVariables|GetCard%20Payload))
              (bind _returnvalue_2 (Game|ConstructObjectfromClass "/Game/Assets/Commands/BP_Command_TransferCards.BP_Command_TransferCards_C" (LocalVariables|GetCard%20Payload) (LocalVariables|GetDestination)))
              (Utilities|Array|Add (LocalVariables|GetOutCommands) _returnvalue_2))))
        (:then_1
          ;;[0 0 0] Create card transfer commands to the foundation piles
          (for _array_element_2 (Variables|/Script/Cards.SolitaireBoard|GetFoundation GameBoard)
            (bind _output_get_3 (LocalVariables|SetDestination (Variables|/Script/Cards.CardPile|GetCardPileComponent _array_element_2)))
            (if (Class|CardPileComponent|CanAccept _output_get_3 (LocalVariables|GetCard%20Payload))
              (bind _returnvalue_3 (Game|ConstructObjectfromClass "/Game/Assets/Commands/BP_Command_TransferCards.BP_Command_TransferCards_C" (LocalVariables|GetCard%20Payload) (LocalVariables|GetDestination)))
              (Utilities|Array|Add (LocalVariables|GetOutCommands) _returnvalue_3))))
        (:then_2
          ;;[0 0 0] Return commands
          (return (LocalVariables|GetOutCommands)))))))

(fn GetCommandDragDrop
  (params (GameBoard :type Solitaire%20Board%20Object%20Reference) (Payload_NEW :type Drag%20Drop%20Payload%20Object%20Reference) (RequestingActor :type Actor%20Object%20Reference))
  (bind _ascard_payload (Utilities|Casting|CastToCardPayload Payload_NEW))
  (LocalVariables|SetCard%20Payload _ascard_payload)
  (bind _returnvalue (Game|ConstructObjectfromClass "/Game/Assets/Commands/BP_Command_TransferCards.BP_Command_TransferCards_C" (LocalVariables|GetCard%20Payload) (Variables|Default|GetCardPileComponent self)))
  (return _returnvalue))

(fn GetDragDropPayload
  (params (GameBoard :type Solitaire%20Board%20Object%20Reference) (RequestingActor :type Actor%20Object%20Reference))
  (bind _ascard (Utilities|Casting|CastToCard RequestingActor))
  ;[0 0 0] Only face-up cards can be picked up in the tableau
  (bind _output_get (LocalVariables|SetRequesting%20Card _ascard))
  (if (not (Variables|/Script/Cards.Card|GetbIsFaceDown _output_get))
    ;[0 0 0] Get the stack of cards on top of the requesting card
    (bind _output_get_2 (LocalVariables|SetCards (Utilities|Array|MakeArray (LocalVariables|GetRequesting%20Card))))
    (Utilities|Array|AppendArray _output_get_2 (Class|CardPileComponent|GetCardsonTopOf (Variables|Default|GetCardPileComponent) (LocalVariables|GetRequesting%20Card)))
    ;[0 0 0] Create the drag and drop payload
    (bind _returnvalue (Game|ConstructObjectfromClass "/Script/Cards.CardPayload"))
    (Class|CardPayload|Initialize _returnvalue (LocalVariables|GetCards) self)
    (return _returnvalue)))

(fn CanAcceptPayload
  (params (GameBoard :type Solitaire%20Board%20Object%20Reference) (Payload :type Drag%20Drop%20Payload%20Object%20Reference) (RequestingActor :type Actor%20Object%20Reference))
  ;[0 0 0] Delegate to card pile ruleset to determine if payload can be accepted
  (bind _ascard_payload (Utilities|Casting|CastToCardPayload Payload)
    (:then
      (return (Class|CardPileComponent|CanAccept (Variables|Default|GetCardPileComponent) _ascard_payload)))
    (:CastFailed
      (return false))))