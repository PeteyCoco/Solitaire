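; Discard pile actor for a solitaire-style card game that only gives out its top card and never accepts payloads or drag-and-drop drops.
; GetDragDropPayload wraps the requesting card in a CardPayload only if it is the top card.
; GetCommands feeds that payload to each tableau and foundation pile's CanAccept check, returning a CommandTransferCard object for every valid destination.
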(event EventBeginPlay)

(event Collision|EventActorBeginOverlap
  (params (OtherActor :type Actor%20Object%20Reference)))

(event EventTick
  (params (DeltaSeconds :type Float%20%28single-precision%29)))

(fn ConstructionScript)

(fn GetCommands
  (params (GameBoard :type Solitaire%20Board%20Object%20Reference) (RequestingActor :type Actor%20Object%20Reference))
  ;[0 0 0] Same behaviour regardless of whether there is a requesting actor or none
  (if (Class|CardPileComponent|IsEmpty (Variables|Default|GetCardPileComponent))
    ;;[0 0 0] Do nothing if the pile is empty
    (return 0)
    (else
      ;;[0 0 0] Make the card payload to transfer
      (bind _ascard_payload (Utilities|Casting|CastToCardPayload (Class|InteractionInterface|GetDragDropPayload GameBoard RequestingActor)))
      (LocalVariables|SetCard%20Payload _ascard_payload)
      ;;[0 0 0] Find all possible card transfers for the payload
      (Utilities|FlowControl|Sequence
        (:then_0
          ;;;[0 0 0] Create card transfer commands to the tableau piles
          (for _array_element (Class|SolitaireBoard|GetTableau GameBoard)
            (bind _output_get (LocalVariables|SetDestination (Variables|/Script/Cards.CardPile|GetCardPileComponent _array_element)))
            (if (Class|CardPileComponent|CanAccept _output_get (LocalVariables|GetCard%20Payload))
              (bind _returnvalue (Game|ConstructObjectfromClass "/Script/Cards.CommandTransferCard" (LocalVariables|GetDestination) (LocalVariables|GetCard%20Payload)))
              (Utilities|Array|Add (LocalVariables|GetOutCommands) _returnvalue))))
        (:then_1
          ;;;[0 0 0] Create card transfer commands to the foundation piles
          (for _array_element_2 (Variables|/Script/Cards.SolitaireBoard|GetFoundation GameBoard)
            (bind _output_get_2 (LocalVariables|SetDestination (Variables|/Script/Cards.CardPile|GetCardPileComponent _array_element_2)))
            (if (Class|CardPileComponent|CanAccept _output_get_2 (LocalVariables|GetCard%20Payload))
              (bind _returnvalue_2 (Game|ConstructObjectfromClass "/Script/Cards.CommandTransferCard" (LocalVariables|GetDestination) (LocalVariables|GetCard%20Payload)))
              (Utilities|Array|Add (LocalVariables|GetOutCommands) _returnvalue_2))))
        (:then_2
          ;;;[0 0 0] Return commands
          (return (LocalVariables|GetOutCommands)))))))

(fn GetCommandDragDrop
  (params (GameBoard :type Solitaire%20Board%20Object%20Reference) (Payload_NEW :type Drag%20Drop%20Payload%20Object%20Reference) (RequestingActor :type Actor%20Object%20Reference))
  ;[0 0 0] No drag-and-drop commands for discard pile
  (return 0))

(fn GetDragDropPayload
  (params (GameBoard :type Solitaire%20Board%20Object%20Reference) (RequestingActor :type Actor%20Object%20Reference))
  ;[0 0 0] Only the top card of the discard pile can be picked up
  (bind _ascard (Utilities|Casting|CastToCard RequestingActor))
  (bind _output_get (LocalVariables|SetRequesting%20Card _ascard))
  (if (== _output_get (Class|CardPileComponent|TopCard (Variables|Default|GetCardPileComponent)))
    ;[0 0 0] Construct the card payload
    (bind _returnvalue (Game|ConstructObjectfromClass "/Script/Cards.CardPayload"))
    (Class|CardPayload|Initialize _returnvalue (Utilities|Array|MakeArray (LocalVariables|GetRequesting%20Card)) self)
    (return _returnvalue)))

(fn CanAcceptPayload
  (params (GameBoard :type Solitaire%20Board%20Object%20Reference) (Payload :type Drag%20Drop%20Payload%20Object%20Reference) (RequestingActor :type Actor%20Object%20Reference))
  ;[0 0 0] Discard pile cannot accept payloads
  (return false))