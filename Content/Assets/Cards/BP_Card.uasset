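; BP_Card is the card actor Blueprint for a card game played on a game board of piles.
; It holds no interaction logic of its own: command, drag-and-drop, payload and acceptance queries all go to the pile that owns it.
; Each query looks up that pile through the GameBoard and passes the card itself as the requesting actor, ignoring the incoming requester.
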(event EventBeginPlay)

(event Collision|EventActorBeginOverlap
  (params (OtherActor :type Actor%20Object%20Reference)))

(event EventTick
  (params (DeltaSeconds :type Float%20%28single-precision%29)))

(fn ConstructionScript)

(fn GetCommands
  (params (GameBoard :type Solitaire%20Board%20Object%20Reference) (RequestingActor :type Actor%20Object%20Reference))
  ;[0 0 0] Cards delegate interactions to their owning piles
  (bind _returnvalue (Class|InteractionInterface|GetCommands(Message) (Class|SolitaireBoard|GetPile GameBoard self) GameBoard self))
  (return _returnvalue))

(fn GetCommandDragDrop
  (params (GameBoard :type Solitaire%20Board%20Object%20Reference) (Payload_NEW :type Drag%20Drop%20Payload%20Object%20Reference) (RequestingActor :type Actor%20Object%20Reference))
  ;[0 0 0] Cards delegate drag-and-drop interactions to their owning piles
  (bind _returnvalue (Class|InteractionInterface|GetCommandDragDrop(Message) (Class|SolitaireBoard|GetPile GameBoard self) GameBoard Payload_NEW self))
  (return _returnvalue))

(fn GetDragDropPayload
  (params (GameBoard :type Solitaire%20Board%20Object%20Reference) (RequestingActor :type Actor%20Object%20Reference))
  ;[0 0 0] Cards always delegate to their owning pile
  (bind _returnvalue (Class|InteractionInterface|GetDragDropPayload(Message) (Class|SolitaireBoard|GetPile GameBoard self) GameBoard self))
  (return _returnvalue))

(fn CanAcceptPayload
  (params (GameBoard :type Solitaire%20Board%20Object%20Reference) (Payload :type Drag%20Drop%20Payload%20Object%20Reference) (RequestingActor :type Actor%20Object%20Reference))
  ;[0 0 0] Card delgates to its owning card pile
  (bind _returnvalue (Class|InteractionInterface|CanAcceptPayload(Message) (Class|SolitaireBoard|GetPile GameBoard self) GameBoard Payload self))
  (return _returnvalue))