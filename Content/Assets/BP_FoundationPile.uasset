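; Solitaire foundation pile actor that takes part in click and drag-and-drop card moves by producing transfer commands.
; Only its top card can be picked up, wrapped in a CardPayload with the pile as origin.
; GetCommands offers moves from the pile to every tableau pile that accepts the card.
; Drops onto the pile become BP_Command_TransferCards when the CardPileComponent, which delegates to its ruleset, accepts the payload.
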(event EventBeginPlay)

(event Collision|EventActorBeginOverlap
  (params (OtherActor :type Actor%20Object%20Reference)))

(event EventTick
  (params (DeltaSeconds :type Float%20%28single-precision%29)))

(fn ConstructionScript)

(fn GetCommands
  (params (GameBoard :type Solitaire%20Board%20Object%20Reference) (RequestingActor :type Actor%20Object%20Reference))
  (if (Class|CardPileComponent|IsEmpty (Variables|Default|GetCardPileComponent))
    ;[0 0 0] Do nothing if the foundation pile is empty
    (return 0)
    (else
      ;[0 0 0] Make the card payload to transfer
      (Utilities|Casting|CastToCardPayload (Class|InteractionInterface|GetDragDropPayload GameBoard RequestingActor))
      (LocalVariables|SetCard%20Payload 0)
      ;[0 0 0] Find all possible card transfers for the payload
      (Utilities|FlowControl|Sequence
        (:then_0
          ;;[0 0 0] Create card transfer commands to the tableau piles
          (for _array_element (Class|SolitaireBoard|GetTableau GameBoard)
            (bind _output_get (LocalVariables|SetDestination (Variables|/Script/Cards.CardPile|GetCardPileComponent _array_element)))
            (if (Class|CardPileComponent|CanAccept _output_get (LocalVariables|GetCard%20Payload))
              (bind _returnvalue (Game|ConstructObjectfromClass "/Game/Assets/Core/Commands/BP_Command_TransferCards.BP_Command_TransferCards_C" (LocalVariables|GetDestination) (LocalVariables|GetCard%20Payload)))
              (Utilities|Array|Add (LocalVariables|GetOutCommands) _returnvalue))))
        (:then_1
          ;;[0 0 0] Return commands
          (return (LocalVariables|GetOutCommands)))))))

(fn GetCommandDragDrop
  (params (GameBoard :type Solitaire%20Board%20Object%20Reference) (Payload_NEW :type Drag%20Drop%20Payload%20Object%20Reference) (RequestingActor :type Actor%20Object%20Reference))
  (bind _ascard_payload (Utilities|Casting|CastToCardPayload Payload_NEW))
  (LocalVariables|SetCard%20Payload _ascard_payload)
  (if (Class|CardPileComponent|CanAccept (Variables|Default|GetCardPileComponent self) (LocalVariables|GetCard%20Payload))
    (bind _returnvalue (Game|ConstructObjectfromClass "/Game/Assets/Core/Commands/BP_Command_TransferCards.BP_Command_TransferCards_C" (Variables|Default|GetCardPileComponent self) (LocalVariables|GetCard%20Payload)))
    (return _returnvalue)))

(fn GetDragDropPayload
  (params (GameBoard :type Solitaire%20Board%20Object%20Reference) (RequestingActor :type Actor%20Object%20Reference))
  ;[0 0 0] Only the top card of the foundation pile is picked up
  (bind _ascard (Utilities|Casting|CastToCard RequestingActor))
  (bind _output_get (LocalVariables|SetRequesting%20Card _ascard))
  (if (== _output_get (Class|CardPileComponent|TopCard (Variables|Default|GetCardPileComponent)))
    ;[0 0 0] Construct the card payload
    (bind _returnvalue (Game|ConstructObjectfromClass "/Script/Cards.CardPayload"))
    (Class|CardPayload|Initialize _returnvalue (Utilities|Array|MakeArray (LocalVariables|GetRequesting%20Card)) self)
    (return _returnvalue)))

(fn CanAcceptPayload
  (params (GameBoard :type Solitaire%20Board%20Object%20Reference) (Payload :type Drag%20Drop%20Payload%20Object%20Reference) (RequestingActor :type Actor%20Object%20Reference))
  ;[0 0 0] Card pile delegates to its ruleset to determine if it can accept the payload
  (bind _ascard_payload (Utilities|Casting|CastToCardPayload Payload)
    (:then
      (return (Class|CardPileComponent|CanAccept (Variables|Default|GetCardPileComponent) _ascard_payload)))
    (:CastFailed
      (return false))))