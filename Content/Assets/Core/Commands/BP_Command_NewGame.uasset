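; BP_Command_NewGame is a macro command that starts a new card game on a given GameBoard.
; On initialization it validates the board, then constructs and queues three sub-commands in order: reset the board, shuffle the deck pile, and deal the cards.
; It returns false without adding any commands if the board is invalid.
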(fn InitializeMacroLogic
  ;[0 0 0] Validate dependencies
  (if (Utilities|IsValid (Variables|Default|GetGameBoard))
    (Utilities|FlowControl|Sequence
      (:then_0
        ;[0 0 0] 1.) Reset the game board
        (bind _returnvalue (Game|ConstructObjectfromClass "/Game/Assets/Core/Commands/BP_Command_ResetBoard.BP_Command_ResetBoard_C" (Variables|Default|GetGameBoard)))
        (Class|SequentialCommand|AddCommand _returnvalue))
      (:then_1
        ;[0 0 0] 2.) Shuffle the deck pile
        (bind _returnvalue_2 (Game|ConstructObjectfromClass "/Script/Cards.CommandShufflePile" (Class|SolitaireBoard|GetDeckPile (Variables|Default|GetGameBoard))))
        (Class|SequentialCommand|AddCommand _returnvalue_2))
      (:then_2
        ;[0 0 0] 3.) Deal the cards
        (bind _returnvalue_3 (Game|ConstructObjectfromClass "/Game/Assets/Core/Commands/BP_Command_DealCards.BP_Command_DealCards_C" (Variables|Default|GetGameBoard)))
        (Class|SequentialCommand|AddCommand _returnvalue_3)
        (return true)))
    (else
      (return false))))