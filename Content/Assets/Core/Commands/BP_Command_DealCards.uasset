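; Macro command that deals the opening Klondike-style solitaire layout from the deck into the tableau piles.
; InitializeMacroLogic queues a transfer command per card, giving each pile one more card than the previous, plus a flip command to reveal each pile's top card.
; A local index walks down from the end of the deck to choose each card as the sub-commands are built.
; It returns false if the GameBoard is invalid.
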(fn InitializeMacroLogic
  ;[0 0 0] Validate dependencies
  (if (Utilities|IsValid (Variables|Default|GetGameBoard))
    ;[0 0 0] Create the macro command
    ;;[0 0 0] Until the tableau piles are full...
    (Utilities|FlowControl|Sequence
      (:then_0
        ;;;[0 0 0] Track the index of the deck card to move
        (LocalVariables|SetDeck%20Card%20Index (- (Class|CardPileComponent|Num (Variables|/Script/Cards.CardPile|GetCardPileComponent (Class|SolitaireBoard|GetDeckPile (Variables|Default|GetGameBoard)))) 1)))
      (:then_1
        ;;;[0 0 0] Deal cards from the deck into the tableau piles
        (for (_ _array_index) (Variables|/Script/Cards.SolitaireBoard|GetTableau (Variables|Default|GetGameBoard))
          (bind _output_get (LocalVariables|SetTableau%20Pile%20Index _array_index))
          (bind _index (Utilities|FlowControl|ForLoopwithBreak 0 _output_get :!label _label)
            (:LoopBody
              (LocalVariables|SetTableau%20Card%20Index _index)
              (Utilities|FlowControl|Sequence
                (:then_0
                  ;;;;[0 0 0] Finish if the deck is out of cards
                  (if (< (LocalVariables|GetDeck%20Card%20Index) 0)
                    (goto _label Break)))
                (:then_1
                  ;;;;[0 0 0] 1.) Get the card at the current deck card index...
                  (LocalVariables|SetCard (Class|CardPileComponent|GetCardatIndex (Variables|/Script/Cards.CardPile|GetCardPileComponent (Class|SolitaireBoard|GetDeckPile (Variables|Default|GetGameBoard))) (LocalVariables|GetDeck%20Card%20Index))))
                (:then_2
                  ;;;;[0 0 0] 2. ) Transfer the card from the deck pile to the tableau pile
                  (bind _returnvalue (Game|ConstructObjectfromClass "/Script/Cards.CardPayload"))
                  (Class|CardPayload|Initialize _returnvalue (Utilities|Array|MakeArray (LocalVariables|GetCard)) (Class|SolitaireBoard|GetDeckPile (Variables|Default|GetGameBoard)))
                  (bind _returnvalue_2 (Game|ConstructObjectfromClass "/Script/Cards.CommandTransferCard" (Variables|/Script/Cards.CardPile|GetCardPileComponent (Utilities|Array|Get(acopy) (Variables|/Script/Cards.SolitaireBoard|GetTableau (Variables|Default|GetGameBoard)) (LocalVariables|GetTableau%20Pile%20Index))) _returnvalue))
                  (Class|SequentialCommand|AddCommand _returnvalue_2))
                (:then_3
                  ;;;;[0 0 0] 3.) Reveal the card if it is the top of the tableau pile
                  (if (== (LocalVariables|GetTableau%20Card%20Index) (LocalVariables|GetTableau%20Pile%20Index))
                    (bind _returnvalue_3 (Game|ConstructObjectfromClass "/Script/Cards.CommandFlipCard" (LocalVariables|GetCard) true))
                    (Class|SequentialCommand|AddCommand _returnvalue_3)))
                (:then_4
                  ;;;;[0 0 0] 4.) Move to the next card in the deck
                  (Math|Integer|DecrementInt (LocalVariables|GetDeck%20Card%20Index)))))))
        ;;;;[0 0 0] Finish macro
        (return true)))
    (else
      (return false))))