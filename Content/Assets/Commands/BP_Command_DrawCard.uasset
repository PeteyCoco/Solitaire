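; BP_Command_DrawCard is a macro command that draws the top card of the deck onto the discard pile, face up.
; InitializeMacroLogic wraps the deck's top card in a CardPayload, then queues a transfer command to the discard pile followed by a flip command.
; It returns false without adding commands when the GameBoard is invalid.
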(fn InitializeMacroLogic
  ;[0 0 0] Validate dependencies
  (if (Utilities|IsValid (Variables|Default|GetGame%20Board))
    ;[0 0 0] Create the macro command
    ;;[0 0 0] For the top card in the discard pile...
    (LocalVariables|SetTop%20Card (Class|CardPileComponent|TopCard (Variables|/Script/Cards.CardPile|GetCardPileComponent (Class|SolitaireBoard|GetDeckPile (Variables|Default|GetGame%20Board)))))
    (Utilities|FlowControl|Sequence
      (:then_0
        ;;;[0 0 0] ...transfer the card to the discard pile
        (bind _returnvalue (Game|ConstructObjectfromClass "/Script/Cards.CardPayload"))
        (Class|CardPayload|Initialize _returnvalue (Utilities|Array|MakeArray (LocalVariables|GetTop%20Card)) (Class|SolitaireBoard|GetDeckPile (Variables|Default|GetGame%20Board)))
        (bind _returnvalue_2 (Game|ConstructObjectfromClass "/Script/Cards.CommandTransferCard" (Variables|/Script/Cards.CardPile|GetCardPileComponent (Class|SolitaireBoard|GetDiscardPile (Variables|Default|GetGame%20Board))) _returnvalue))
        (Class|SequentialCommand|AddCommand _returnvalue_2))
      (:then_1
        ;;;[0 0 0] ... and flip the card face up
        (bind _returnvalue_3 (Game|ConstructObjectfromClass "/Script/Cards.CommandFlipCard" (LocalVariables|GetTop%20Card)))
        (Class|SequentialCommand|AddCommand _returnvalue_3)
        (return true)))
    (else
      (return false))))