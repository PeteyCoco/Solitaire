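; Macro command that resets the game board by returning every card to the deck pile, face down.
; When initialized with a valid GameBoard, it walks the board's cards in reverse order and queues two sub-commands per card.
; A transfer command moves a single-card payload from its current pile to the deck, then a flip command turns it face down.
; Initialization returns false if the GameBoard is invalid.
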(fn InitializeMacroLogic
  ;[0 0 0] Validate dependencies
  (if (Utilities|IsValid (Variables|Default|GetGame%20Board))
    ;[0 0 0] Create the macro command
    ;;[0 0 0] For each card on the game board...
    (bind _arrayelement (Utilities|Array|ReverseforEachLoop (Class|SolitaireBoard|GetCards (Variables|Default|GetGame%20Board)))
      (:LoopBody
        (LocalVariables|SetCard _arrayelement)
        (Utilities|FlowControl|Sequence
          (:then_0
            ;;;[0 0 0] ...transfer the card to the deck pile
            (bind _returnvalue (Game|ConstructObjectfromClass "/Script/Cards.CardPayload"))
            (Class|CardPayload|Initialize _returnvalue (Utilities|Array|MakeArray (LocalVariables|GetCard)) (Class|SolitaireBoard|GetPile (Variables|Default|GetGame%20Board) (LocalVariables|GetCard)))
            (bind _returnvalue_2 (Game|ConstructObjectfromClass "/Script/Cards.CommandTransferCard" (Variables|/Script/Cards.CardPile|GetCardPileComponent (Class|SolitaireBoard|GetDeckPile (Variables|Default|GetGame%20Board))) _returnvalue))
            (Class|SequentialCommand|AddCommand _returnvalue_2))
          (:then_1
            ;;;[0 0 0] ... and flip the card face down
            (bind _returnvalue_3 (Game|ConstructObjectfromClass "/Script/Cards.CommandFlipCard" (LocalVariables|GetCard) false))
            (Class|SequentialCommand|AddCommand _returnvalue_3))))
      (:Completed
        (return true)))
    (else
      (return false))))