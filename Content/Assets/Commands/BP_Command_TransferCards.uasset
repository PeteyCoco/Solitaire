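; Macro command that transfers a set of cards to a destination in the card game.
; On initialization it splits the payload into single-card payloads that keep the original origin.
; Each one becomes a CommandTransferCard sub-command aimed at the same destination and is added to the macro.
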(fn InitializeMacroLogic
  ;[0 0 0] Create a single card transfer command for each card in the payload
  (for _array_element (Class|CardPayload|GetCards (Variables|Default|GetPayload))
    (bind _returnvalue (Game|ConstructObjectfromClass "/Script/Cards.CardPayload"))
    (Class|CardPayload|Initialize _returnvalue (Utilities|Array|MakeArray _array_element) (Variables|/Script/Cards.CardPayload|GetOrigin (Variables|Default|GetPayload)))
    (bind _returnvalue_2 (Game|ConstructObjectfromClass "/Script/Cards.CommandTransferCard" (Variables|Default|GetDestination) _returnvalue))
    (Class|SequentialCommand|AddCommand _returnvalue_2))
  (return true))