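; A macro command that reshuffles the deck by moving the discard pile back into the deck pile on the game board.
; On initialization it walks the discard pile in reverse order and, for each card, queues a transfer command with a single-card payload, then a flip-face-down command.
; It builds only these sub-commands, with no randomization, and fails if the game board is invalid.
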(fn InitializeMacroLogic
  ;[0 0 0] Validate dependencies
  (if (Utilities|IsValid (Variables|Default|GetGameBoard))
    ;[0 0 0] Create the macro command
    ;;[0 0 0] For each card in the discard pile...
    (bind _returnvalue (Class|CardPileComponent|GetAllCards (Variables|/Script/Cards.CardPile|GetCardPileComponent (Class|SolitaireBoard|GetDiscardPile (Variables|Default|GetGameBoard)))))
    (bind _arrayelement (Utilities|Array|ReverseforEachLoop _returnvalue)
      (:LoopBody
        (LocalVariables|SetCard _arrayelement)
        (Utilities|FlowControl|Sequence
          (:then_0
            ;;;[0 0 0] ...transfer the card from the discard pile to the deck pile
            (bind _returnvalue_2 (Game|ConstructObjectfromClass "/Script/Cards.CardPayload"))
            (Class|CardPayload|Initialize _returnvalue_2 (Utilities|Array|MakeArray (LocalVariables|GetCard)) (Class|SolitaireBoard|GetDiscardPile (Variables|Default|GetGameBoard)))
            (bind _returnvalue_3 (Game|ConstructObjectfromClass "/Script/Cards.CommandTransferCard" (Variables|/Script/Cards.CardPile|GetCardPileComponent (Class|SolitaireBoard|GetDeckPile (Variables|Default|GetGameBoard))) _returnvalue_2))
            (Class|SequentialCommand|AddCommand _returnvalue_3))
          (:then_1
            ;;;[0 0 0] ... and flip the card face down
            (bind _returnvalue_4 (Game|ConstructObjectfromClass "/Script/Cards.CommandFlipCard" (LocalVariables|GetCard) false))
            (Class|SequentialCommand|AddCommand _returnvalue_4))))
      (:Completed
        (return true)))
    (else
      (return false))))